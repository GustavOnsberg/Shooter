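; Player controller that respawns the player character after its pawn is destroyed.
; On BeginPlay it binds to the controlled Player_BP's OnDestroyed event and saves that pawn's transform as the spawn point.
; When destruction fires, it waits briefly, spawns and possesses a new Player_BP there, adjusting for collision.
; It then calls Respawn to rebind and re-save the transform, so the cycle repeats.
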(event Custom|Respawn
  (bind _asplayer_bp (Utilities|Casting|CastToPlayer_BP (Pawn|GetControlledPawn)))
  (Game|BindEventtoOnDestroyed _asplayer_bp (delegate Custom|OnDestroy))
  (Variables|Default|SetSpawnTransform (Transformation|GetActorTransform (Pawn|GetControlledPawn))))

(event Custom|OnDestroy
  (Utilities|FlowControl|Delay 2.0)
  (bind _returnvalue (Game|SpawnActorfromClass "/Game/Blueprints/Player/Player_BP.Player_BP_C" (Variables|Default|GetSpawnTransform) "AdjustIfPossibleButAlwaysSpawn" 0 0))
  (Pawn|Possess self _returnvalue)
  (CallFunction|Respawn))

(event EventBeginPlay
  (bind _asplayer_bp (Utilities|Casting|CastToPlayer_BP (Pawn|GetControlledPawn)))
  (Game|BindEventtoOnDestroyed _asplayer_bp (delegate Custom|OnDestroy))
  (Variables|Default|SetSpawnTransform (Transformation|GetActorTransform (Pawn|GetControlledPawn))))

(fn ConstructionScript)