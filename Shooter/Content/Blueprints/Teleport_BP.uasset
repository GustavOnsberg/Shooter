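; Teleporter actor that moves any actor overlapping it to a configurable destination transform, including its scale.
; With Randomness enabled, each location and rotation axis gets a random offset within plus or minus the matching additive value; otherwise the transform applies exactly.
; The Construction Script places the TeleportPoint component at the destination in world space.
; Overlaps are not filtered by actor type.
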(event EventBeginPlay)

(event EventActorBeginOverlap
  (params (OtherActor :type Actor%20Object%20Reference))
  (bind _teleportpointtransform (Variables|Default|GetTeleportPointTransform))
  (bind _randomlocationadditive (Variables|Default|GetRandomLocationAdditive))
  (bind _randomrotationadditive (Variables|Default|GetRandomRotationAdditive))
  (if (Variables|Default|GetRandomness)
    (Transformation|SetActorTransform OtherActor (Math|Transform|MakeTransform (Math|Vector|MakeVector (+ (Math|Random|RandomFloatinRange (- 0.0 (.x _randomlocationadditive)) (.x _randomlocationadditive)) (.x (.location _teleportpointtransform))) (+ (Math|Random|RandomFloatinRange (- 0.0 (.y _randomlocationadditive)) (.y _randomlocationadditive)) (.y (.location _teleportpointtransform))) (+ (Math|Random|RandomFloatinRange (- 0.0 (.z _randomlocationadditive)) (.z _randomlocationadditive)) (.z (.location _teleportpointtransform)))) (Math|Rotator|MakeRotator (+ (Math|Random|RandomFloatinRange (- 0.0 (.roll _randomrotationadditive)) (.roll _randomrotationadditive)) (.roll (.rotation _teleportpointtransform))) (+ (Math|Random|RandomFloatinRange (- 0.0 (.pitch _randomrotationadditive)) (.pitch _randomrotationadditive)) (.pitch (.rotation _teleportpointtransform))) (+ (Math|Random|RandomFloatinRange (- 0.0 (.yaw _randomrotationadditive)) (.yaw _randomrotationadditive)) (.yaw (.rotation _teleportpointtransform)))) (.scale _teleportpointtransform)))
    (else
      (Transformation|SetActorTransform OtherActor (Variables|Default|GetTeleportPointTransform)))))

(event EventTick
  (params (DeltaSeconds :type Float%20%28single-precision%29)))

(fn ConstructionScript
  (Transformation|SetWorldTransform (Variables|Default|GetTeleportPoint) (Variables|Default|GetTeleportPointTransform) false false))