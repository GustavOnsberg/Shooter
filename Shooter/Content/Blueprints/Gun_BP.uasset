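; Gun Blueprint that chooses its Gun at BeginPlay through a rarity-weighted random roll over six tiers, Common to Legendary.
; It compares the roll with cumulative PickPoints thresholds, then takes a random entry from that tier's array on GameModeBase_BP.
; The threshold tests read `sum <= Picked`, so with non-negative weights only Common can be chosen, and lower rolls set nothing.
; Array indices roll up to Length inclusive, one past the last element.
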(event EventBeginPlay
  (bind _returnvalue (Game|GetGameMode))
  (bind _commonpickpoints (Variables|Default|GetCommonPickPoints))
  (bind _uncommonpickpoints (Variables|Default|GetUncommonPickPoints))
  (bind _rarepickpoints (Variables|Default|GetRarePickPoints))
  (bind _varyrarepickpoints (Variables|Default|GetVaryRarePickPoints))
  (bind _superrarepickpoints (Variables|Default|GetSuperRarePickPoints))
  (bind _commonpickpoints_2 (Variables|Default|GetCommonPickPoints))
  (bind _uncommonpickpoints_2 (Variables|Default|GetUncommonPickPoints))
  (bind _rarepickpoints_2 (Variables|Default|GetRarePickPoints))
  (bind _varyrarepickpoints_2 (Variables|Default|GetVaryRarePickPoints))
  (bind _superrarepickpoints_2 (Variables|Default|GetSuperRarePickPoints))
  (bind _legendarypickpoints (Variables|Default|GetLegendaryPickPoints))
  (bind _returnvalue_2 (+ _commonpickpoints_2 _uncommonpickpoints_2 _rarepickpoints_2 _varyrarepickpoints_2 _superrarepickpoints_2 _legendarypickpoints))
  (Variables|Default|SetTotalPickPoints _returnvalue_2)
  (Variables|Default|SetPicked (Math|Random|RandomIntegerinRange 0 _returnvalue_2))
  (if (<= _commonpickpoints (Variables|Default|GetPicked))
    (bind _asgame_mode_base_bp (Utilities|Casting|CastToGameModeBase_BP _returnvalue))
    (Variables|Default|SetGun (Utilities|Array|Get(acopy) (Variables|/Game/Blueprints/GameModeBase_BP.GameModeBase_BP_C|GetCommon%20Guns _asgame_mode_base_bp) (Math|Random|RandomIntegerinRange 0 (Utilities|Array|Length (Variables|/Game/Blueprints/GameModeBase_BP.GameModeBase_BP_C|GetCommon%20Guns _asgame_mode_base_bp)))))
    (elif (<= (+ _commonpickpoints _uncommonpickpoints) (Variables|Default|GetPicked))
      (bind _asgame_mode_base_bp_2 (Utilities|Casting|CastToGameModeBase_BP _returnvalue))
      (Variables|Default|SetGun (Utilities|Array|Get(acopy) (Variables|/Game/Blueprints/GameModeBase_BP.GameModeBase_BP_C|GetUncommon%20Guns _asgame_mode_base_bp_2) (Math|Random|RandomIntegerinRange 0 (Utilities|Array|Length (Variables|/Game/Blueprints/GameModeBase_BP.GameModeBase_BP_C|GetUncommon%20Guns _asgame_mode_base_bp_2)))))
      (elif (<= (+ _commonpickpoints _uncommonpickpoints _rarepickpoints) (Variables|Default|GetPicked))
        (bind _asgame_mode_base_bp_3 (Utilities|Casting|CastToGameModeBase_BP _returnvalue))
        (Variables|Default|SetGun (Utilities|Array|Get(acopy) (Variables|/Game/Blueprints/GameModeBase_BP.GameModeBase_BP_C|GetRare%20Guns _asgame_mode_base_bp_3) (Math|Random|RandomIntegerinRange 0 (Utilities|Array|Length (Variables|/Game/Blueprints/GameModeBase_BP.GameModeBase_BP_C|GetRare%20Guns _asgame_mode_base_bp_3)))))
        (elif (<= (+ _commonpickpoints _uncommonpickpoints _rarepickpoints _varyrarepickpoints) (Variables|Default|GetPicked))
          (bind _asgame_mode_base_bp_4 (Utilities|Casting|CastToGameModeBase_BP _returnvalue))
          (Variables|Default|SetGun (Utilities|Array|Get(acopy) (Variables|/Game/Blueprints/GameModeBase_BP.GameModeBase_BP_C|GetVary%20Rare%20Guns _asgame_mode_base_bp_4) (Math|Random|RandomIntegerinRange 0 (Utilities|Array|Length (Variables|/Game/Blueprints/GameModeBase_BP.GameModeBase_BP_C|GetVary%20Rare%20Guns _asgame_mode_base_bp_4)))))
          (elif (<= (+ _commonpickpoints _uncommonpickpoints _rarepickpoints _varyrarepickpoints _superrarepickpoints) (Variables|Default|GetPicked))
            (bind _asgame_mode_base_bp_5 (Utilities|Casting|CastToGameModeBase_BP _returnvalue))
            (Variables|Default|SetGun (Utilities|Array|Get(acopy) (Variables|/Game/Blueprints/GameModeBase_BP.GameModeBase_BP_C|GetSuper%20Rare%20Guns _asgame_mode_base_bp_5) (Math|Random|RandomIntegerinRange 0 (Utilities|Array|Length (Variables|/Game/Blueprints/GameModeBase_BP.GameModeBase_BP_C|GetSuper%20Rare%20Guns _asgame_mode_base_bp_5)))))
            (elif (<= (+ _commonpickpoints _uncommonpickpoints _rarepickpoints _varyrarepickpoints _superrarepickpoints (Variables|Default|GetLegendaryPickPoints)) (Variables|Default|GetPicked))
              (bind _asgame_mode_base_bp_6 (Utilities|Casting|CastToGameModeBase_BP _returnvalue))
              (Variables|Default|SetGun (Utilities|Array|Get(acopy) (Variables|/Game/Blueprints/GameModeBase_BP.GameModeBase_BP_C|GetLegendary%20Guns _asgame_mode_base_bp_6) (Math|Random|RandomIntegerinRange 0 (Utilities|Array|Length (Variables|/Game/Blueprints/GameModeBase_BP.GameModeBase_BP_C|GetLegendary%20Guns _asgame_mode_base_bp_6))))))))))))

(fn ConstructionScript)