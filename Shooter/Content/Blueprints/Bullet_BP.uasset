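; Bullet projectile actor that delivers base and special damage to whatever it hits.
; Start receives the shot's speed, damage settings and owning pawn, storing them and setting the projectile movement's initial speed.
; Hit prints the struck bone name, passes base and special-damage values to the other actor through DamageMessage, then destroys the bullet.
; Splash damage settings and the owning pawn are stored but not used here.
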(event Collision|EventHit
  (params (MyComp :type Primitive%20Component%20Object%20Reference) (Other :type Actor%20Object%20Reference) (OtherComp :type Primitive%20Component%20Object%20Reference) (bSelfMoved :type Boolean) (HitLocation :type Vector :default "0, 0, 0") (HitNormal :type Vector :default "0, 0, 0") (NormalImpulse :type Vector :default "0, 0, 0") (Hit :type Hit%20Result%20Structure%20%28by%20ref%29))
  (Development|PrintString (Utilities|String|ToString(Name) (.HitBoneName (Collision|BreakHitResult Hit))))
  (Class|DamageBPIF|Damage(Message) Other (Variables|Default|GetBaseDamage) (Variables|Default|GetSpecialDamageType) (Variables|Default|GetSpecialDamageTypeAffectChance) (Variables|Default|GetSpecialDamageTypeDamagePerSec) (Variables|Default|GetSpecialDamageTypeDamageTime))
  (Actor|DestroyActor))

(fn ConstructionScript)

(fn Start
  (params (Speed :type Float%20%28single-precision%29) (BaseDamage :type Integer) (SplashDamage :type Boolean) (SplashDamageRange :type Float%20%28single-precision%29) (SplashDamageMax :type Integer) (SplashDamageMin :type Integer) (SpecialDamageTypeDamagePerSec :type Integer) (SpecialDamageTypeAffectChance :type Float%20%28single-precision%29) (SpecialDamageTypeDamageTime :type Float%20%28single-precision%29) (OwningPawn :type Pawn%20Object%20Reference) (SpecialDamgeType :type GunDamagesTypeList%20Enum))
  (Variables|/Script/Engine.ProjectileMovementComponent|SetInitialSpeed (Variables|Default|GetProjectileMovement) Speed)
  (Variables|Default|SetBaseDamage BaseDamage)
  (Variables|Default|SetSplashDamage SplashDamage)
  (Variables|Default|SetSplashDamageRange SplashDamageRange)
  (Variables|Default|SetSplashDamageMax SplashDamageMax)
  (Variables|Default|SetSplashDamageMin SplashDamageMin)
  (Variables|Default|SetSpecialDamageTypeDamagePerSec SpecialDamageTypeDamagePerSec)
  (Variables|Default|SetSpecialDamageTypeAffectChance SpecialDamageTypeAffectChance)
  (Variables|Default|SetSpecialDamageTypeDamageTime SpecialDamageTypeDamageTime)
  (Variables|Default|SetOwningPawn OwningPawn)
  (Variables|Default|SetSpecialDamageType SpecialDamgeType))